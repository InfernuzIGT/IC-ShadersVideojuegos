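; BP_Fruit is an interactive fruit actor for a shader intro demo, with a configurable mesh, adjustable slicing and highlight/select states.
; A dynamic material instance receives an Edge scalar, stepped and clamped by Add/RemoveSlice, and a Brightness scalar for dim, highlighted and selected states.
; Select plays a timeline that lerps the actor horizontally toward the world's vertical origin axis; Unselect reverses it and leaves the fruit highlighted.
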(event Custom|Refresh%20Slice
  (Rendering|Material|SetScalarParameterValue (Variables|Default|GetMaterial) "Edge" (Variables|Default|GetSlice%20Value) :!class /Script/Engine.MaterialInstanceDynamic))

(event EventBeginPlay
  (bind _returnvalue (Transformation|GetActorLocation))
  (bind _sm_fruit (Variables|Default|GetSM_Fruit))
  (Components|StaticMesh|SetStaticMesh _sm_fruit (Variables|Default|GetMesh))
  (bind _returnvalue_2 (Rendering|Material|CreateDynamicMaterialInstance _sm_fruit 0 (Rendering|Material|GetMaterial _sm_fruit 0) "None" :!class /Script/Engine.PrimitiveComponent))
  (Variables|Default|SetMaterial _returnvalue_2)
  (CallFunction|RefreshSlice)
  (Variables|Default|SetStart%20Location _returnvalue)
  (Variables|Default|SetEnd%20Location (+ _returnvalue (* (Math|Vector|GetUnitDirection(Vector) _returnvalue (Math|Vector|MakeVector 0.0 0.0 (.Z (Math|Vector|BreakVector _returnvalue)))) (Math|Float|MakeLiteralFloat 1e+02))))
  (CallFunction|ChangeHighlightState false))

(event EventAddSlice
  (Variables|Default|SetSlice%20Value (Math|Float|Clamp(Float) (+ (Variables|Default|GetSlice%20Value) (Math|Float|MakeLiteralFloat 0.05))))
  (CallFunction|RefreshSlice))

(event EventRemoveSlice
  (Variables|Default|SetSlice%20Value (Math|Float|Clamp(Float) (- (Variables|Default|GetSlice%20Value) (Math|Float|MakeLiteralFloat 0.05))))
  (CallFunction|RefreshSlice))

(event EventUnselect
  (CallFunction|ChangeHighlightState true)
  (bind _lerp (Timeline|Timeline%20Zoom Reverse)
    (:Update
      (Transformation|SetActorLocation (Math|Vector|Lerp(Vector) (Variables|Default|GetStart%20Location) (Variables|Default|GetEnd%20Location) _lerp) false false))))

(event EventSelect
  (Rendering|Material|SetScalarParameterValue (Variables|Default|GetMaterial) "Brightness" 1.0 :!class /Script/Engine.MaterialInstanceDynamic)
  (bind _lerp (Timeline|Timeline%20Zoom Play)
    (:Update
      (Transformation|SetActorLocation (Math|Vector|Lerp(Vector) (Variables|Default|GetStart%20Location) (Variables|Default|GetEnd%20Location) _lerp) false false))))

(event EventChangeHighlightState
  (params (bShow :type Boolean))
  (Rendering|Material|SetScalarParameterValue (Variables|Default|GetMaterial) "Brightness" (select bShow 0.5 0.1) :!class /Script/Engine.MaterialInstanceDynamic))

(fn ConstructionScript
  (Components|StaticMesh|SetStaticMesh (Variables|Default|GetSM_Fruit) (Variables|Default|GetMesh)))