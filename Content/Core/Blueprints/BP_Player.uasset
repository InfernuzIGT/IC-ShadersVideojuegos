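; Player Blueprint that inspects and manipulates objects in view through first-person camera aiming and a HUD reticle.
; A per-tick camera line trace caches the hit actor until the trace misses, toggling its highlight and the reticle.
; Holding right mouse selects the target and turns mouse look into object rotation.
; The mouse wheel messages the target to add or remove slices, and Escape quits the game.
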(event EventBeginPlay
  (bind _returnvalue (UserInterface|CreateWidget "/Game/Core/Widgets/WBP_HUD.WBP_HUD_C"))
  (bind _output_get (Variables|Default|SetWBP%20HUD _returnvalue))
  (UserInterface|Viewport|AddtoViewport _output_get 0))

(event EventTick
  (params (DeltaSeconds :type Float%20%28single-precision%29))
  (bind _wbp_hud (Variables|Default|GetWBP%20HUD))
  (bind _camera (Variables|Default|GetCamera))
  (bind _returnvalue (Transformation|GetWorldLocation _camera))
  (bind (_outhit _returnvalue_2) (Collision|LineTraceByChannel _returnvalue (+ _returnvalue (* (Math|Vector|GetForwardVector _camera) (Math|Float|MakeLiteralFloat 1e+03))) "TraceTypeQuery1" false 0 "None"))
  (if _returnvalue_2
    (Utilities|IsValid (Variables|Default|GetHit%20Actor)
      (:Is%20Not%20Valid
        (bind _output_get (Variables|Default|SetHit%20Actor (.HitActor (Collision|BreakHitResult _outhit))))
        (Default|ChangeReticleState _wbp_hud true)
        (Class|BPIFruit|ChangeHighlightState(Message) _output_get true)))
    (else
      (Utilities|IsValid (Variables|Default|GetHit%20Actor)
        (:Is%20Valid
          (Class|BPIFruit|ChangeHighlightState(Message) (Variables|Default|GetHit%20Actor) false)
          (Variables|Default|SetHit%20Actor 0)
          (Default|ChangeReticleState _wbp_hud false))))))

(event Input|MouseEvents|MouseWheelUp
  (params (Key :type Key%20Structure :default "None"))
  (bind _hit_actor (Variables|Default|GetHit%20Actor))
  (:Pressed
    (Utilities|IsValid _hit_actor
      (:Is%20Valid
        (Class|BPIFruit|AddSlice(Message) _hit_actor)))))

(event Input|KeyboardEvents|Escape
  (params (Key :type Key%20Structure :default "None"))
  (:Pressed
    (Game|QuitGame 0 "Quit" false)))

(event Input|MouseEvents|MouseWheelDown
  (params (Key :type Key%20Structure :default "None"))
  (bind _hit_actor (Variables|Default|GetHit%20Actor))
  (:Pressed
    (Utilities|IsValid _hit_actor
      (:Is%20Valid
        (Class|BPIFruit|RemoveSlice(Message) _hit_actor)))))

(event Input|MouseEvents|RightMouseButton
  (params (Key :type Key%20Structure :default "None"))
  (bind _wbp_hud (Variables|Default|GetWBP%20HUD))
  (bind _hit_actor (Variables|Default|GetHit%20Actor))
  (:Pressed
    (Variables|Default|SetbRotationMode true)
    (Utilities|IsValid _hit_actor
      (:Is%20Valid
        (Class|BPIFruit|Select(Message) _hit_actor)
        (Default|Select _wbp_hud))))
  (:Released
    (Variables|Default|SetbRotationMode false)
    (Utilities|IsValid _hit_actor
      (:Is%20Valid
        (Class|BPIFruit|Unselect(Message) _hit_actor)
        (Default|Unselect _wbp_hud)))))

(event Input|MouseEvents|Mouse2D
  (params (AxisValue :type Vector :default "0, 0, 0"))
  (bind (_x _y) (Math|Vector|BreakVector AxisValue))
  (bind _returnvalue (Game|GetPlayerController 0))
  (bind _returnvalue_2 (Math|Float|MakeLiteralFloat 5.0))
  (bind _hit_actor (Variables|Default|GetHit%20Actor))
  (bind (_deltax _deltay) (Class|PlayerController|GetInputMouseDelta _returnvalue))
  (if (Variables|Default|GetbRotationMode)
    (Utilities|IsValid _hit_actor
      (:Is%20Valid
        (Class|Actor|AddActorWorldRotation _hit_actor (Math|Rotator|MakeRotator 0.0 (* _deltay _returnvalue_2 -1.0) (* _deltax _returnvalue_2)))))
    (else
      (Pawn|Input|AddControllerYawInput _x)
      (Pawn|Input|AddControllerPitchInput (* _y -1.0)))))

(fn ConstructionScript)